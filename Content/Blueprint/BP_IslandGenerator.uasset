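; BP_IslandGenerator is an actor that procedurally generates an island from a seeded, irregular circular spline and a PCG graph.
; GenerateIslandSpline passes a seed-derived value to the graph's Seed parameter, picks a random radius, and rebuilds the spline with configurable point count and deviation.
; It runs this and triggers PCG generation in both the construction script, where generation is forced, and BeginPlay, where it is not.
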(event EventBeginPlay
  (CallFunction|GenerateIslandSpline)
  (PCG|Generate (Variables|Default|GetPCG) false))

(fn ConstructionScript
  (CallFunction|GenerateIslandSpline)
  (PCG|Generate (Variables|Default|GetPCG) true))

(fn GenerateIslandSpline
  (bind _seed (Variables|Default|GetSeed))
  (Class|PCGGraphParametersHelpers|SetInt32Parameter (Variables|/Script/PCG.PCGComponent|GetGraphInstance (Variables|Default|GetPCG)) "Seed" (Class|KismetMathLibrary|RandomIntegerfromStream _seed 255))
  (bind _output_get (Variables|Default|SetRadius (Math|Random|RandomFloatinRangefromStream _seed 5e+03 8e+03)))
  (bind _returnvalue (Class|SplineGenerator|GenerateCircularSplineVector3D (Variables|Default|GetSplinePointsNum) _output_get _seed (Variables|Default|GetPointDeviation)))
  (Spline|SetSplinePoints (Variables|Default|GetSpline) _returnvalue "Local" true))